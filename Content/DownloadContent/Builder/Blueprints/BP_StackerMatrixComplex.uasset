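; Builder actor that generates a 3D grid of static mesh components in its construction script when Generate is set.
; Spacing comes from a fixed offset or fixed area, with optional centering, index-scaled rotation and scale steps, and seeded random transforms.
; Meshes cycle or are picked randomly, then SpecificMeshes entries override individual indices.
; PlacePermanentCopies spawns each component as a standalone StaticMeshActor with the same mesh and world transform.
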(fn `PlacePermanentCopies`
  (for _array_element (`self.MeshComps`)
    (bind _returnvalue (`|SpawnActorFromClass` "/Script/Engine.StaticMeshActor" (`SceneComponent.K2_GetComponentToWorld` _array_element) "AlwaysSpawn" "OverrideRootScale" null null))
    (`StaticMeshComponent.SetStaticMesh` (`StaticMeshActor.StaticMeshComponent` _returnvalue) (`StaticMeshComponent.StaticMesh` _array_element))))

(fn `UserConstructionScript`
  (locals (Offset :type "Vector Structure") (Base :type "Vector Structure") (pIndex :type Integer))
  (bind _locationbase (`self.LocationBase`))
  (bind _seed (`self.Seed`))
  (if (`self.Generate`)
    (`KismetArrayLibrary.Array_Clear` (`self.MeshComps`))
    (`|ExecutionSequence`
      (:`then_0`
        (set `local.Offset` (select `/Game/DownloadContent/Builder/Blueprints/EMatrixPlacement` (`self.Mode`) :`NewEnumerator0` (`self.LocationOffset`) :`NewEnumerator1` (`KismetMathLibrary.MakeVector` (/ (.x (`self.Area`)) (`KismetMathLibrary.FMax` (`KismetMathLibrary.Conv_IntToDouble` (- (`self.Rows`) 1)) 1.0)) (/ (.y (`self.Area`)) (`KismetMathLibrary.FMax` (`KismetMathLibrary.Conv_IntToDouble` (- (`self.Columns`) 1)) 1.0)) (/ (.z (`self.Area`)) (`KismetMathLibrary.FMax` (`KismetMathLibrary.Conv_IntToDouble` (- (`self.Levels`) 1)) 1.0)))))
        (set `local.Base` (`KismetMathLibrary.SelectVector` (+ (select `/Game/DownloadContent/Builder/Blueprints/EMatrixPlacement` (`self.Mode`) :`NewEnumerator0` (/ (`KismetMathLibrary.MakeVector` (* (.x (`self.LocationOffset`)) (`KismetMathLibrary.Conv_IntToDouble` (- (`self.Rows`) 1))) (* (.y (`self.LocationOffset`)) (`KismetMathLibrary.Conv_IntToDouble` (- (`self.Columns`) 1))) (* (.z (`self.LocationOffset`)) (`KismetMathLibrary.Conv_IntToDouble` (- (`self.Levels`) 1)))) -2.0) :`NewEnumerator1` (/ (`self.Area`) -2.0)) _locationbase) _locationbase (`self.Center`))))
      (:`then_1`
        (for _index (range (`self.Levels`))
          (for _index_2 (range (`self.Rows`))
            (for _index_3 (range (`self.Columns`))
              (bind _returnvalue (+ _index_3 (* _index_2 (`self.Columns`)) (* _index (* (`self.Columns`) (`self.Rows`)))))
              (bind _returnvalue_2 (`AddComponent|NODE_AddStaticMeshComponent-1` :`RelativeTransform` (`/Game/DownloadContent/Builder/Blueprints/BP_FuncLib.CombineTransform` (`KismetMathLibrary.MakeTransform` (+ (`KismetMathLibrary.MakeVector` (* _index_2 (.x (`local.Offset`))) (* _index_3 (.y (`local.Offset`))) (* _index (.z (`local.Offset`)))) (`local.Base`)) (`KismetMathLibrary.ComposeRotators` (* (`self.RotationOffset`) _returnvalue) (`self.RotationBase`)) (+ (* (`self.ScaleOffset`) _returnvalue) (`self.ScaleBase`))) (`KismetMathLibrary.MakeTransform` (`/Game/DownloadContent/Builder/Blueprints/BP_FuncLib.RandomVectorSeeded` (`self.MinRandomLocation`) (`self.MaxRandomLocation`) _seed) (`/Game/DownloadContent/Builder/Blueprints/BP_FuncLib.RandomRotSeeded` (`self.MinRandomRotation`) (`self.MaxRandomRotation`) _seed) (`/Game/DownloadContent/Builder/Blueprints/BP_FuncLib.RandomVectorSeeded` (`self.MinRandomScale`) (`self.MaxRandomScale`) _seed)))))
              (switch `/Game/DownloadContent/Builder/Blueprints/ESelect` (`self.MeshSelection`)
                (:`NewEnumerator0`
                  (`StaticMeshComponent.SetStaticMesh` _returnvalue_2 (`|GetArrayItem` (`self.Mesh`) (`local.pIndex`)))
                  (set `local.pIndex` (mod (+ (`local.pIndex`) 1) (`KismetArrayLibrary.Array_Length` (`self.Mesh`)))))
                (:`NewEnumerator1`
                  (`StaticMeshComponent.SetStaticMesh` _returnvalue_2 (`/Game/DownloadContent/Builder/Blueprints/BP_MacroLib.RandomItemSeeded` (`self.Mesh`) (`self.Seed`)))))
              (`KismetArrayLibrary.Array_Add` (`self.MeshComps`) _returnvalue_2)))))
      (:`then_2`
        (for _array_element (`self.SpecificMeshes`)
          (bind (_index_4 _mesh _offset _rot _scale) (break `/Game/DownloadContent/Builder/Blueprints/S_IndexMesh` _array_element))
          (if (and (> (`KismetArrayLibrary.Array_Length` (`self.MeshComps`)) _index_4) (> _index_4 -1))
            (bind _output (`|GetArrayItem` (`self.MeshComps`) _index_4))
            (`StaticMeshComponent.SetStaticMesh` _output _mesh)
            (`SceneComponent.K2_SetRelativeTransform` _output (`KismetMathLibrary.MakeTransform` (+ (`SceneComponent.RelativeLocation` _output) _offset) _rot _scale) false false)))))))